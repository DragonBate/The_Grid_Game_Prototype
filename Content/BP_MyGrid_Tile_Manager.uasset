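; Grid tile manager actor that, as shown, only positions two corner meshes marking the bounds of a grid.
; The construction script snaps the actor location and the GridEnd3D offset point to 300-unit steps.
; It places Cube one step below the start and StaticMesh one step beyond the end in X and Y, keeping the snapped Z.
; The event graph holds no active logic.
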(event EventBeginPlay)

(event Collision|EventActorBeginOverlap
  (params (OtherActor :type Actor%20Object%20Reference)))

(event EventTick
  (params (DeltaSeconds :type Float%20%28single-precision%29)))

(fn ConstructionScript
  (bind _returnvalue (Class|GSFuncLib|VectorRoundto (Transformation|GetActorLocation) 3e+02))
  (Transformation|SetWorldLocation (Variables|Default|GetCube) (Math|Vector|MakeVector (- (.X (Math|Vector|BreakVector _returnvalue)) 3e+02) (- (.Y (Math|Vector|BreakVector _returnvalue)) 3e+02) (.Z (Math|Vector|BreakVector _returnvalue))) false true)
  (bind _returnvalue_2 (Class|GSFuncLib|VectorRoundto (+ (Variables|Default|GetGridEnd3D) (Transformation|GetActorLocation)) 3e+02))
  (Transformation|SetWorldLocation (Variables|Default|GetStaticMesh) (Math|Vector|MakeVector (- (.X (Math|Vector|BreakVector _returnvalue_2)) -3e+02) (- (.Y (Math|Vector|BreakVector _returnvalue_2)) -3e+02) (.Z (Math|Vector|BreakVector _returnvalue_2))) false true))