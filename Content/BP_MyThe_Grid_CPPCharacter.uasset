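; First-person character Blueprint for a grid building game, used to test placing buildings on Grid_Tile actors.
; Tick line-traces from the camera with debug drawing, opening a gate only while a Grid_Tile is hit.
; Spawn input passes through that gate, prints the tile's CanPlace result with affordability hardcoded true, then calls BuildWall with the selected class name.
; BeginPlay creates the test HUD; debug keys adjust GameState currency and power, while selection-cycling logic is unconnected.
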(event EventTick
  (params (DeltaSeconds :type Float%20%28single-precision%29))
  (bind _returnvalue (Class|KismetSystemLibrary|MakeLiteralBool true))
  (bind _buildingclassed (Variables|Default|GetBuildingClassed))
  (bind _selectedbuilding (Variables|Default|GetSelectedBuilding))
  (bind _firstpersoncameracomponent (Variables|Default|GetFirstPersonCameraComponent))
  (bind _item (Utilities|Array|Get(acopy) _buildingclassed _selectedbuilding))
  (bind _returnvalue_2 (Transformation|GetWorldLocation _firstpersoncameracomponent))
  (bind _returnvalue_3 (Utilities|String|StringToName _item))
  (bind _outhit (Collision|LineTraceByChannel _returnvalue_2 (+ (* (Math|Vector|GetForwardVector _firstpersoncameracomponent) 5000) _returnvalue_2) "TraceTypeQuery1" false 0 "ForOneFrame"))
  (if (== (Utilities|GetClass (.hitactor _outhit)) "/Script/The_Grid_CPP.Grid_Tile")
    (Utilities|FlowControl|Gate true) ; enters at Open
    (else
      (Utilities|FlowControl|Gate true) ; enters at Close
    )))

(event EventBeginPlay
  ;[1 1 1] Init
  (bind _returnvalue (UserInterface|CreateWidget "/Game/TestingHud.TestingHud_C" (Game|GetPlayerController 0) self))
  (UserInterface|Viewport|AddtoViewport _returnvalue 0)
  (bind _asgrid_game_state (Utilities|Casting|CastToGrid_GameState (Game|GetGameState)))
  (Variables|Default|SetGS_Ref _asgrid_game_state))

(event Input|ActionEvents|InputActionSpawn
  (params (Key :type Key%20Structure :default "AnyKey"))
  (bind _returnvalue (Class|KismetSystemLibrary|MakeLiteralBool true))
  (bind _buildingclassed (Variables|Default|GetBuildingClassed))
  (bind _selectedbuilding (Variables|Default|GetSelectedBuilding))
  (bind _item (Utilities|Array|Get(acopy) _buildingclassed _selectedbuilding))
  (bind _returnvalue_2 (Utilities|String|StringToName _item))
  (:Pressed
    (Utilities|FlowControl|Gate true
      (:Exit
        (bind _asgrid_tile (Utilities|Casting|CastToGrid_Tile (.hitactor (stale EventTick _outhit))))
        (bind _returnvalue_3 (Class|GridTile|CanPlace _asgrid_tile _returnvalue_2 _returnvalue))
        (Development|PrintString (Class|KismetStringLibrary|BuildStringBool (Utilities|String|ToString(Name) _returnvalue_2) " - Can Place: " _returnvalue_3))
        (if (and _returnvalue_3 _returnvalue)
          (Class|GridTile|BuildWall _asgrid_tile _returnvalue_2))))))

(event Input|KeyboardEvents|E
  (params (Key :type Key%20Structure :default "AnyKey")))

(event Input|KeyboardEvents|LeftBracket
  (params (Key :type Key%20Structure :default "AnyKey"))
  (:Pressed
    (Class|GridGameState|AddtoPower (Variables|Default|GetGS_Ref) 1)))

(event Input|KeyboardEvents|RightBracket
  (params (Key :type Key%20Structure :default "AnyKey"))
  (:Pressed
    (Class|GridGameState|AddtoPower (Variables|Default|GetGS_Ref) -1)))

(event Input|KeyboardEvents|9
  (params (Key :type Key%20Structure :default "AnyKey"))
  (:Pressed
    (Class|GridGameState|AddtoCurrency (Variables|Default|GetGS_Ref) 1)))

(event Input|KeyboardEvents|0
  (params (Key :type Key%20Structure :default "AnyKey"))
  (:Pressed
    (Class|GridGameState|AddtoCurrency (Variables|Default|GetGS_Ref) -1)))

(event Input|MouseEvents|MouseWheelDown
  (params (Key :type Key%20Structure :default "AnyKey"))
  ;[1 1 1] Class Selection
)

(event Input|MouseEvents|MouseWheelUp
  (params (Key :type Key%20Structure :default "AnyKey"))
  ;[1 1 1] Class Selection
)

(fn ConstructionScript)